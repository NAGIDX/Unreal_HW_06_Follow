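; BP_GameMode is a game mode that runs a minute and second countdown and pauses the game when time runs out.
; Tick feeds a one-second Delay, which throttles the decrement of Second to about once per second.
; When Second drops below zero it wraps to 59 and takes one from Minute, or, with no minutes left, resets to zero and pauses the game.
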(event `self.ReceiveTick`
  (params (DeltaSeconds :type "Float (single-precision)"))
  ;[1 0.05471 0] TimeCount System
  ;;[1 1 1] Sec-=1
  (`KismetSystemLibrary.Delay` 1.0)
  (bind _output_get (set `self.Second` (- (`self.Second`) 1)))
  ;;[1 1 1] If Sec =0 Then Sec=59
  (if (< _output_get 0)
    (set `self.Second` 59)
    ;;[1 1 1] If Min > 0 Then Min-=1
    (if (> (`self.Minute`) 0)
      (set `self.Minute` (- (`self.Minute`) 1))
      (else
        ;;[1 1 1] If Min ==0 and Sec ==59 Then Sec == 0  Set Game Paused
        (if (== (`self.Second`) 59)
          (set `self.Second` 0)
          (`GameplayStatics.SetGamePaused` true))))))

(fn `UserConstructionScript`)